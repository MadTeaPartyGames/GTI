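; Actor component that finds the item the player is looking at and flags it as interactable through gameplay tags.
; GetItem runs an object line trace, using the controller's focal location, height offset and control rotation to place it.
; FocusCheck reads the hit actor's tags via interface messages, toggles its highlight and the player's CanInteract tag, and reports whether it is collectable.
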(fn `FocusCheck`
  (params (InteractItem :type "Object Object Reference") (Condition :type Boolean) (PlayerTagContainer :type "GameplayTagContainer Structure (by ref)"))
  (returns (Collectable :type Boolean))
  ;[0.2623 0 1] Used to check the output InteractItem from GetItem. This will determine if the actor is interactive or a collectable, and react accordingly.
  (if Condition
    (bind _tagcontainer (message `/Game/GTI_Core/BPI_GTI_Interface.GetTags` InteractItem))
    (if (`BlueprintGameplayTagLibrary.HasTag` _tagcontainer (struct :`TagName` "Item.Interactive") true)
      (bind _output_get (set `self.InteractItem` InteractItem))
      (`BlueprintGameplayTagLibrary.AddGameplayTag` PlayerTagContainer (struct :`TagName` "GTI.Action.CanInteract"))
      (message `/Game/GTI_Core/BPI_GTI_Interface.ItemHighlight` _output_get)
      (return (`BlueprintGameplayTagLibrary.HasTag` _tagcontainer (struct :`TagName` "Item.Collectable") true))
      (else
        (`|ExecutionSequence` :!label _label
          (:`then_0`
            (bind _interactitem (`self.InteractItem`)
              (:`then`
                (message `/Game/GTI_Core/BPI_GTI_Interface.ItemRemoveHighlight` _interactitem))
              (:`else`)))
          (:`then_1`
            (if (`BlueprintGameplayTagLibrary.HasTag` PlayerTagContainer (struct :`TagName` "GTI.Action.CanInteract") true)
              (bind _returnvalue (`BlueprintGameplayTagLibrary.RemoveGameplayTag` PlayerTagContainer (struct :`TagName` "GTI.Action.CanInteract")))
              (if _returnvalue
                (return (`BlueprintGameplayTagLibrary.HasTag` _tagcontainer (struct :`TagName` "Item.Collectable") true))))))))
    (else
      (goto _label))))

(fn `GetItem`
  (params (PlayerController :type "PlayerController Object Reference") (TraceDistance :type "Float (double-precision)") (HeightOffset :type "Float (double-precision)") (DrawDebugType :type "EDrawDebugTrace Enum" :default "None"))
  (returns (InteractItem :type "Object Object Reference") (ReturnValue :type Boolean))
  (bind _returnvalue (`KismetMathLibrary.MakeVector` (.x (`PlayerController.GetFocalLocation` PlayerController)) (.y (`PlayerController.GetFocalLocation` PlayerController)) (+ (.z (`PlayerController.GetFocalLocation` PlayerController)) HeightOffset)))
  ;[0.2623 0 1] Simple LineTraceForObject returning the Hit Actor and Blocking Hit.
  (bind _outhit (`KismetSystemLibrary.LineTraceSingleForObjects` :`Start` _returnvalue :`End` (+ _returnvalue (* (`KismetMathLibrary.GetForwardVector` (`Controller.GetControlRotation` PlayerController)) TraceDistance)) :`ObjectTypes` (`|MakeArray` "ObjectTypeQuery1" "ObjectTypeQuery2" "ObjectTypeQuery4" :!type "EObjectTypeQuery Enum") :`DrawDebugType` DrawDebugType))
  (bind (_bblockinghit _binitialoverlap _time _distance _location _impactpoint _normal _impactnormal _physmat _hitactor) (`GameplayStatics.BreakHitResult` _outhit))
  (return _hitactor _bblockinghit))