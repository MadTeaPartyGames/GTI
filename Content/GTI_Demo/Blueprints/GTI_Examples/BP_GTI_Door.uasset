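; Example interactable door, derived from BP_GTI_ItemParent, whose locked, open, moving and key color states are driven by Gameplay Tags.
; Server interaction unlocks it when PlayerController tags match its key, otherwise swings it via timeline, opening away from the player.
; The construction script previews open rotation, lock light and key color in editor.
; Opening, closing and lock sounds play at the mesh, and highlight events toggle custom depth.
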(event `self.ReceiveBeginPlay`
  ;[0.2623 0 1] Set up Event bindings, adding extra highlight to meshes.
  (add `self.OnHighlight` (delegate `ExtraHighlight`))
  (add `self.OnRemoveHighlight` (delegate `RemoveExtraHighlight`)))

(event `LockedSound`
  ;[0.2623 0 1] Multicast RPC to play door lock and unlock sounds. Doing it this way since a door would be audible to everyone IRL.
  (`GameplayStatics.PlaySoundAtLocation` (`BlueprintMapLibrary.Map_Find` (`self.DoorSounds`) "Locked") (`SceneComponent.K2_GetComponentLocation` (`self.StaticMesh`)) (struct) 1.0 1.0 0.0 null null null null))

(event `ExtraHighlight`
  ;[0.2623 0 1] Set up Event bindings, adding extra highlight to meshes.
  (`PrimitiveComponent.SetRenderCustomDepth` (`self.Door`) true))

(event `RemoveExtraHighlight`
  ;[0.2623 0 1] Set up Event bindings, adding extra highlight to meshes.
  (`PrimitiveComponent.SetRenderCustomDepth` (`self.Door`) false))

(event `UnlockSound`
  ;[0.2623 0 1] Multicast RPC to play door lock and unlock sounds. Doing it this way since a door would be audible to everyone IRL.
  (`GameplayStatics.PlaySoundAtLocation` (`BlueprintMapLibrary.Map_Find` (`self.DoorSounds`) "Unlock") (`SceneComponent.K2_GetComponentLocation` (`self.StaticMesh`)) (struct) 1.0 1.0 0.0 null null null null))

(event `/Game/GTI_Core/BPI_GTI_Interface.ItemInteractServer`
  (params (PlayerController :type "PlayerController Object Reference"))
  (bind _tagcontainer (`self.TagContainer`))
  (bind _relativerotation (`SceneComponent.RelativeRotation` (`self.StaticMesh`)))
  ;[0.2623 0 1] Event ItemInteractServer: Overriding the event from the parent BP_GTI_ItemParent class to drive the door. First check is for a locked door, and if the PlayerController has a matching key to unlock the door. Rotation values are then set based on direction the pawn is facing (door always opens away from player).
  (if (`BlueprintGameplayTagLibrary.HasTag` (`self.TagContainer`) (struct :`TagName` "Item.Door.Locked") true)
    (bind _tagcontainer_2 (message `/Game/GTI_Core/BPI_GTI_Interface.GetTags` PlayerController))
    (if (`BlueprintGameplayTagLibrary.HasAnyTags` _tagcontainer_2 (`self.TagContainer`) true)
      (if (`BlueprintGameplayTagLibrary.DoesContainerMatchTagQuery` (`self.TagContainer`) (`self.KeyColorQuery`))
        (`self.UnlockSound`)
        (`BlueprintGameplayTagLibrary.RemoveGameplayTag` (`self.TagContainer`) (struct :`TagName` "Item.Door.Locked")))
      (else
        (`self.LockedSound`)))
    (elif (not (`BlueprintGameplayTagLibrary.HasTag` _tagcontainer (struct :`TagName` "Item.Door.Moving") true))
      (`BlueprintGameplayTagLibrary.AddGameplayTag` _tagcontainer (struct :`TagName` "Item.Door.Moving"))
      (set `self.OriginalRot` _relativerotation)
      (if (`KismetMathLibrary.NearlyEqual_FloatFloat` (.yaw _relativerotation) 0.0 1.0)
        (`self.IsPlayerFacingDoorFront` PlayerController
          (:`true`
            (set `self.DoorRotYaw` -90.0))
          (:`false`
            (set `self.DoorRotYaw` 90.0)))
        (else
          (`/Engine/EditorBlueprintResources/StandardMacros.CompareFloat` (.yaw (`SceneComponent.RelativeRotation` (`self.StaticMesh`)))
            (:`>`
              (set `self.DoorRotYaw` -90.0))
            (:`<`
              (set `self.DoorRotYaw` 90.0)))))
      (`self.RotateDoor`))))

(event `RotateDoor`
  (bind _originalrot (`self.OriginalRot`))
  (bind _tagcontainer (`self.TagContainer`))
  (bind _tagcontainer_2 (`self.TagContainer`))
  (bind _returnvalue (`BlueprintGameplayTagLibrary.HasTag` _tagcontainer (struct :`TagName` "Item.Door.Open") true))
  ;[0.2623 0 1] Event RotateDoor: Timeline to drive door rotation based on the yaw that was set in Event ItemInteractServer.
  (bind (_direction _alpha) (`Timeline|RotateDoor_TL` :!via `PlayFromStart`)
    (:`Update`
      (`SceneComponent.K2_SetRelativeRotation` (`self.StaticMesh`) (`KismetMathLibrary.RLerp` _originalrot (`KismetMathLibrary.MakeRotator` (.roll _originalrot) (.pitch _originalrot) (+ (.yaw _originalrot) (`self.DoorRotYaw`))) _alpha) false false)
      (if _returnvalue
        (`/Engine/EditorBlueprintResources/StandardMacros.DoOnce` false :!label _label
          (:`Completed`
            (`GameplayStatics.PlaySoundAtLocation` (`BlueprintMapLibrary.Map_Find` (`self.DoorSounds`) "Closing") (`SceneComponent.K2_GetComponentLocation` (`self.StaticMesh`)) (struct) 1.0 1.0 0.0 null null null null)))
        (else
          (`/Engine/EditorBlueprintResources/StandardMacros.DoOnce` false :!label _label_2
            (:`Completed`
              (`GameplayStatics.PlaySoundAtLocation` (`BlueprintMapLibrary.Map_Find` (`self.DoorSounds`) "Opening") (`SceneComponent.K2_GetComponentLocation` (`self.StaticMesh`)) (struct) 1.0 1.0 0.0 null null null null))))))
    (:`Finished`
      (`BlueprintGameplayTagLibrary.RemoveGameplayTag` _tagcontainer (struct :`TagName` "Item.Door.Moving"))
      (if _returnvalue
        (`BlueprintGameplayTagLibrary.RemoveGameplayTag` _tagcontainer_2 (struct :`TagName` "Item.Door.Open"))
        (goto _label :!via `Reset`)
        (else
          (`BlueprintGameplayTagLibrary.AddGameplayTag` _tagcontainer_2 (struct :`TagName` "Item.Door.Open"))
          (goto _label_2 :!via `Reset`))))))

(fn `UserConstructionScript`
  ;[0.2623 0 1] Checking for tags to determine if the door should be open, if it is locked, and what color to set the light to if it is. This is in the construction script so changes can be seen real-time in the editor.
  (`parent.UserConstructionScript`)
  (`|ExecutionSequence`
    (:`then_0`
      (for _array_element (`BlueprintGameplayTagLibrary.BreakGameplayTagContainer` (`self.TagContainer`))
        (if (`BlueprintGameplayTagLibrary.MatchesTag` _array_element (struct :`TagName` "Item.Door.Locked") true)
          (`SceneComponent.SetVisibility` (`self.Light`) true false))))
    (:`then_1`
      (for _array_element_2 (`BlueprintGameplayTagLibrary.BreakGameplayTagContainer` (`self.TagContainer`))
        (`|SwitchGameplayTag` _array_element_2
          (:`Item.Key.Blue`
            (set `self.LightColor` (struct :`G` 0.038916 :`B` 1.0 :`A` 1.0)))
          (:`Item.Key.Green`
            (set `self.LightColor` (struct :`R` 0.084105 :`G` 0.973958 :`B` 0.039259 :`A` 1.0)))
          (:`Item.Key.Red`
            (set `self.LightColor` (struct :`R` 0.963542 :`G` 0.048352 :`B` 0.019593 :`A` 1.0)))
          (:`Item.Key.Yellow`
            (set `self.LightColor` (struct :`R` 1.0 :`G` 0.921582 :`A` 1.0))))
        (`LightComponent.SetLightColor` (`self.Light`) (`self.LightColor`) true)))
    (:`then_2`
      (if (`BlueprintGameplayTagLibrary.HasTag` (`self.TagContainer`) (struct :`TagName` "Item.Door.Open") true)
        (`SceneComponent.K2_SetRelativeRotation` (`self.StaticMesh`) (`KismetMathLibrary.MakeRotator` (.roll (`SceneComponent.RelativeRotation` (`self.StaticMesh`))) (.pitch (`SceneComponent.RelativeRotation` (`self.StaticMesh`))) (+ (.yaw (`SceneComponent.RelativeRotation` (`self.StaticMesh`))) -90.0)) false false)))))