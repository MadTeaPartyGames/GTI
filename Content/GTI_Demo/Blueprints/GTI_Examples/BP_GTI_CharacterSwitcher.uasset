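; Interactable character switcher that swaps the interacting player between first-person and third-person pawns, with a skeletal mesh looping a walk animation as its display.
; The overridden ItemInteractServer event reads the controlled pawn's gameplay tags to choose the opposite character class.
; It spawns that class at the Sphere component's location and rotation, destroys the old pawn and possesses the new one, toggling input around the swap.
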(event `self.ReceiveBeginPlay`
  (`SkeletalMeshComponent.PlayAnimation` (`self.SkeletalMesh`) "/Game/Characters/Mannequins/Animations/Quinn/MF_Walk_Fwd.MF_Walk_Fwd" true))

(event `/Game/GTI_Core/BPI_GTI_Interface.ItemInteractServer`
  (params (PlayerController :type "PlayerController Object Reference"))
  (bind _playercontroller (`self.PlayerController`))
  (bind _returnvalue (`Controller.K2_GetPawn` (`self.PlayerController`)))
  (bind _returnvalue_2 (`Controller.K2_GetPawn` (`self.PlayerController`)))
  (bind _returnvalue_3 (`KismetMathLibrary.MakeTransform` (.location (`SceneComponent.K2_GetComponentToWorld` (`self.Sphere`))) (.rotation (`SceneComponent.K2_GetComponentToWorld` (`self.Sphere`)))))
  ;[0.2623 0 1] Event overriding ItemInteractServer. Checking the tag on the player pawn for the type, spawning the other pawn type, and then destroy old pawn and possess new.
  (bind _output_get (set `self.PlayerController` PlayerController))
  (`self.DisableInput` _returnvalue_2 _output_get)
  (bind _tagcontainer (message `/Game/GTI_Core/BPI_GTI_Interface.GetTags` _returnvalue_2))
  (`|SwitchGameplayTagContainer` _tagcontainer
    (:`(GameplayTags=((TagName="Pawn.Player.FP")))`
      (bind _returnvalue_4 (`|SpawnActorFromClass` "/Game/GTI_Demo/Blueprints/BP_ThirdPersonCharacter.BP_ThirdPersonCharacter_C" _returnvalue_3 "Undefined" "OverrideRootScale" null null))
      (`self.K2_DestroyActor` _returnvalue)
      (`Controller.Possess` _playercontroller _returnvalue_4))
    (:`(GameplayTags=((TagName="Pawn.Player.TP")))`
      (bind _returnvalue_5 (`|SpawnActorFromClass` "/Game/GTI_Demo/Blueprints/FirstPersonCharacter.FirstPersonCharacter_C" _returnvalue_3 "Undefined" "OverrideRootScale" null null))
      (`self.K2_DestroyActor` _returnvalue)
      (`Controller.Possess` _playercontroller _returnvalue_5)))
  (`self.EnableInput` _returnvalue _playercontroller))

(fn `UserConstructionScript`
  (`parent.UserConstructionScript`))