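; Parent item actor for interactable, collectable objects, with separate client and server interface events for interaction and collection.
; Each event calls a matching dispatcher as an extension hook; client events also play sounds at the Arrow's location, and server collection destroys the actor.
; Highlight events toggle custom depth on the static and skeletal meshes only when the Item.Highlight gameplay tag is present.
; Helper functions add, remove and return the item's tags.
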(event `/Game/GTI_Core/BPI_GTI_Interface.ItemInteractClient`
  ;[0.2623 0 1] Interface Event ItemInteractClient: This will call the dispatcher, and play a sound at the location.
  (`self.OnItemInteractClient`)
  (`GameplayStatics.PlaySoundAtLocation` (`self.InteractSound`) (`SceneComponent.K2_GetComponentLocation` (`self.Arrow`)) (struct) 1.0 1.0 0.0 null null null null))

(event `/Game/GTI_Core/BPI_GTI_Interface.ItemHighlight`
  ;[0.2623 0 1] Interface Event ItemHighlight: Check item to see if it should be highlighted, set RenderCustomDepth, and call dispatcher Event.
  (if (`BlueprintGameplayTagLibrary.HasTag` (`self.TagContainer`) (struct :`TagName` "Item.Highlight") true)
    (`PrimitiveComponent.SetRenderCustomDepth` (`self.SkeletalMesh`) true)
    (`PrimitiveComponent.SetRenderCustomDepth` (`self.StaticMesh`) true)
    (`self.OnHighlight`)))

(event `/Game/GTI_Core/BPI_GTI_Interface.ItemCollectClient`
  ;[0.2623 0 1] Interface Event ItemCollectClient: This will play a sound at the location and call dispatcher Event.
  (`GameplayStatics.PlaySoundAtLocation` (`self.CollectSound`) (`SceneComponent.K2_GetComponentLocation` (`self.Arrow`)) (struct) 1.0 1.0 0.0 null null null null)
  (`self.OnItemCollectClient`))

(event `/Game/GTI_Core/BPI_GTI_Interface.ItemRemoveHighlight`
  ;[0.2623 0 1] Interface Event ItemRemoveHighlight: Check item to see if it should be highlighted, set RenderCustomDepth, and call dispatcher Event.
  (if (`BlueprintGameplayTagLibrary.HasTag` (`self.TagContainer`) (struct :`TagName` "Item.Highlight") true)
    (`PrimitiveComponent.SetRenderCustomDepth` (`self.StaticMesh`) false)
    (`PrimitiveComponent.SetRenderCustomDepth` (`self.SkeletalMesh`) false)
    (`self.OnRemoveHighlight`)))

(event `/Game/GTI_Core/BPI_GTI_Interface.ItemInteractServer`
  (params (PlayerController :type "PlayerController Object Reference"))
  ;[0.2623 0 1] Interface Event ItemInteractServer: Has PlayerController input to ensure events are triggered by the correct player in multiplayer, and call dispatcher Event.
  (`self.OnItemInteractServer`))

(event `/Game/GTI_Core/BPI_GTI_Interface.ItemCollectServer`
  (params (PlayerController :type "PlayerController Object Reference"))
  ;[0.2623 0 1] Interface Event ItemCollectServer: Has PlayerController input to ensure events are triggered by the correct player in multiplayer, call dispatcher Event, and destroy item.
  (`self.OnItemCollectServer`)
  (`self.K2_DestroyActor`))

(fn `AddTag`
  (params (TagToAdd :type "GameplayTag Structure"))
  (returns (ReturnValue :type Boolean))
  (`BlueprintGameplayTagLibrary.AddGameplayTag` (`self.TagContainer`) TagToAdd)
  (return true))

(fn `GetTags`
  (returns (TagContainer :type "GameplayTagContainer Structure"))
  (return (`self.TagContainer`)))

(fn `RemoveTag`
  (params (TagToRemove :type "GameplayTag Structure"))
  (returns (ReturnValue :type Boolean))
  (bind _returnvalue (`BlueprintGameplayTagLibrary.RemoveGameplayTag` (`self.TagContainer`) TagToRemove))
  (return _returnvalue))

(fn `UserConstructionScript`)