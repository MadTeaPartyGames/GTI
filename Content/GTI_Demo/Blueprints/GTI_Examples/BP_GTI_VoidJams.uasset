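; Interactable GTI demo item that plays the VoidsMindJam music if the player has the Item.VoidJams tag, or a "No" sound otherwise.
; Overrides ItemInteractClient to check gameplay tags fetched from the player controller and play the chosen sound at the mesh.
; A DoOnce guards the music, and removing the Item.Interactive tag then ends interaction.
; BeginPlay applies the MetalRef material to the mesh.
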(event `self.ReceiveBeginPlay`
  ;[0.2623 0 1] Event BeginPlay: Setting material based on reference.
  (`PrimitiveComponent.SetMaterial` (`self.StaticMesh`) 0 (`|ConvertAsset` (`self.MetalRef`))))

(event `/Game/GTI_Core/BPI_GTI_Interface.ItemInteractClient`
  ;[0.2623 0 1] Event ItemInteractClient override. Getting player tags to check for Item.VoidJams and playing sound accordingly. Once the music loop starts, item is no longer interactive.
  (bind _tagcontainer (message `/Game/GTI_Core/BPI_GTI_Interface.GetTags` (`GameplayStatics.GetPlayerController` 0)))
  (if (`BlueprintGameplayTagLibrary.HasTag` _tagcontainer (struct :`TagName` "Item.VoidJams") true)
    (set `self.InteractSound` "/Game/GTI_Demo/Sound/Music/SC_GTI_VoidsMindJam.SC_GTI_VoidsMindJam")
    (`/Engine/EditorBlueprintResources/StandardMacros.DoOnce` false
      (:`Completed`
        (`GameplayStatics.PlaySoundAtLocation` (`self.InteractSound`) (`SceneComponent.K2_GetComponentLocation` (`self.StaticMesh`)) (struct) 1.0 1.0 0.0 null null null null)
        (`BlueprintGameplayTagLibrary.RemoveGameplayTag` (`self.TagContainer`) (struct :`TagName` "Item.Interactive"))))
    (else
      (bind _output_get (set `self.InteractSound` "/Game/GTI_Demo/Sound/SFX/Cues/SC_GTI_No.SC_GTI_No"))
      (`GameplayStatics.PlaySoundAtLocation` _output_get (`SceneComponent.K2_GetComponentLocation` (`self.StaticMesh`)) (struct) 1.0 1.0 0.0 null null null null))))

(fn `UserConstructionScript`
  (`parent.UserConstructionScript`))