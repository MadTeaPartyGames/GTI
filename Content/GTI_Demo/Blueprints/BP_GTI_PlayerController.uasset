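; Player controller for the GTI demo that drives gameplay-tag-based item interaction, creates the HUD and handles demo hotkeys.
; Each tick, BPGTIACInteract traces for items, runs a focus check and pushes the result to HUD events instead of bindings.
; Interact requires the CanInteract tag, then re-traces in client and server RPCs, calling collect or interact interface messages by item tag.
; The client triggers item FX; the server then removes the tag.
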(event `self.ReceiveBeginPlay`
  ;[0.2623 0 1] Event BeginPlay: Setting up widget used for the HUD. Since we don't care for splitscreen in this example, we can just plug in GetPlayerController to handle networked play.
  (bind _returnvalue (`|CreateWidget` "/Game/GTI_Demo/UI/WBP_GTI_HUD.WBP_GTI_HUD_C" (`GameplayStatics.GetPlayerController` 0)))
  (bind _output_get (set `self.HUD` _returnvalue))
  (`UserWidget.AddToViewport` _output_get 0))

(event `self.ReceiveTick`
  (params (DeltaSeconds :type "Float (single-precision)"))
  ;[0.2623 0 1] Event Tick: Yes, this is running on tick. This is a lightweight check, it is less overhead than a timer, and we do not want to do any delays on tick. This will allow for better accuracy in replication. Async trace in C++ would give best performance.
  (`self.InteractCheck`) ; See GTI InteractGraph
)

(event `Key|Escape`
  (params (Key :type "Key Structure"))
  ;[0.2623 0 1] Basic demo inputs
  (:`Pressed`
    (`KismetSystemLibrary.QuitGame` (`GameplayStatics.GetPlayerController` 0) "Quit")))

(event `InputAction|Interact`
  (params (Key :type "Key Structure"))
  ;[0.2623 0 1] InputAction Interact: Default bound to E. This will check for our tag, and if the player can, it will call the RPC Event ClientInteract.
  (:`Pressed`
    (if (`BlueprintGameplayTagLibrary.HasTag` (`self.TagContainer`) (struct :`TagName` "GTI.Action.CanInteract") true)
      (`self.ClientInteract`))))

(event `Key|One`
  (params (Key :type "Key Structure"))
  ;[0.2623 0 1] Basic demo inputs
  (:`Pressed`
    (`KismetSystemLibrary.ExecuteConsoleCommand` "stat fps" null)))

(event `Key|Two`
  (params (Key :type "Key Structure"))
  ;[0.2623 0 1] Basic demo inputs
  (:`Pressed`
    (`KismetSystemLibrary.ExecuteConsoleCommand` "stat unit" null)))

(event `Key|R`
  (params (Key :type "Key Structure"))
  (:`Pressed`
    (`/Engine/EditorBlueprintResources/ActorMacros.Switch Has Authority`
      (:`Authority`
        (bind _asgame_mode (cast `GameMode` (`GameplayStatics.GetGameMode`)))
        (`GameMode.RestartGame` _asgame_mode)))))

(event `InteractCheck`
  ;[0.2623 0 1] Event InteractCheck: RPC Executes on Owning Client. This is the trace that runs on tick to check the hit item if it is interactive, and if it should highlight the item. Then the HUD will be updated by calling Events in the WBP. This is more efficient that using bindings or Tick in the WBP.
  (bind (_interactitem _returnvalue) (`/Game/GTI_Core/BP_GTI_AC.GetItem` (`self.BP_GTI_AC_Interact`) self 200.0 64.0 "None"))
  (bind _collectable (`/Game/GTI_Core/BP_GTI_AC.FocusCheck` (`self.BP_GTI_AC_Interact`) _interactitem _returnvalue (`self.TagContainer`)))
  (bind _hud (`self.HUD`)
    (:`then`
      (`/Game/GTI_Demo/UI/WBP_GTI_HUD.UpdateCrosshair_Event` _hud)
      (`/Game/GTI_Demo/UI/WBP_GTI_HUD.UpdateInteractText_Event` _hud _collectable))
    (:`else`)))

(event `ClientInteract`
  ;[0.2623 0 1] Event ClientInteract: RPC Executes on Owning Client. This will fire a single trace on the client to check the current item for its type, call the interface function based on this to play to appropriate FX for the item, then call Event ServerInteract.
  (bind _interactitem (`/Game/GTI_Core/BP_GTI_AC.GetItem` (`self.BP_GTI_AC_Interact`) self 200.0 64.0 "None"))
  (bind _tagcontainer (message `/Game/GTI_Core/BPI_GTI_Interface.GetTags` _interactitem))
  (if (`BlueprintGameplayTagLibrary.HasTag` _tagcontainer (struct :`TagName` "Item.Collectable") true)
    (message `/Game/GTI_Core/BPI_GTI_Interface.ItemCollectClient` _interactitem)
    (else
      (message `/Game/GTI_Core/BPI_GTI_Interface.ItemInteractClient` _interactitem)))
  (`self.ServerInteract`))

(event `ServerInteract`
  ;[0.2623 0 1] Event ServerInteract: RPC Executes on Server, Reliable. This will fire a single trace on the server to check the current item for its type, call the interface function based on this, then remove the tag GTI.Action.CanInteract to reset the player to be able to interact with another item.
  (bind _interactitem (`/Game/GTI_Core/BP_GTI_AC.GetItem` (`self.BP_GTI_AC_Interact`) self 200.0 64.0 "None"))
  (bind _tagcontainer (message `/Game/GTI_Core/BPI_GTI_Interface.GetTags` _interactitem))
  (if (`BlueprintGameplayTagLibrary.HasTag` _tagcontainer (struct :`TagName` "Item.Collectable") true)
    (message `/Game/GTI_Core/BPI_GTI_Interface.ItemCollectServer` _interactitem self)
    (else
      (message `/Game/GTI_Core/BPI_GTI_Interface.ItemInteractServer` _interactitem self)))
  (`BlueprintGameplayTagLibrary.RemoveGameplayTag` (`self.TagContainer`) (struct :`TagName` "GTI.Action.CanInteract")))

(fn `AddTag`
  (params (TagToAdd :type "GameplayTag Structure"))
  (returns (ReturnValue :type Boolean))
  (`BlueprintGameplayTagLibrary.AddGameplayTag` (`self.TagContainer`) TagToAdd)
  (return true))

(fn `GetTags`
  (returns (TagContainer :type "GameplayTagContainer Structure"))
  (return (`self.TagContainer`)))

(fn `ItemCollectClient`
  (return))

(fn `ItemCollectServer`
  (params (PlayerController :type "PlayerController Object Reference")))

(fn `ItemHighlight`
  (return))

(fn `ItemInteractClient`
  (return))

(fn `ItemInteractServer`
  (params (PlayerController :type "PlayerController Object Reference"))
  (return))

(fn `ItemRemoveHighlight`
  (return))

(fn `RemoveTag`
  (params (TagToRemove :type "GameplayTag Structure"))
  (returns (ReturnValue :type Boolean))
  (bind _returnvalue (`BlueprintGameplayTagLibrary.RemoveGameplayTag` (`self.TagContainer`) TagToRemove))
  (return _returnvalue))

(fn `UserConstructionScript`)