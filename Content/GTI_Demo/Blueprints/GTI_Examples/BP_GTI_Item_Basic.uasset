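; BP_GTI_Item_Basic is a basic example item for the GTI demo that picks its static mesh material from its gameplay tags.
; The construction script switches on the tag container, applying a metal material for highlighted interactive items and a gold one when they are also collectable.
; Materials are held as soft references to keep the actor light.
; The event graph adds no behavior beyond calling the parent's BeginPlay.
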(event `self.ReceiveBeginPlay`
  (`parent.ReceiveBeginPlay`))

(fn `UserConstructionScript`
  (bind _staticmesh (`self.StaticMesh`))
  ;[0.2623 0 1] Switch on Gameplay Tag Container to set the material based on it being interactive or collectable. Soft refs are used to avoid this just taking up 14MB in the actor for no real reason.
  (`parent.UserConstructionScript`)
  (`|SwitchGameplayTagContainer` (`self.TagContainer`)
    (:`(GameplayTags=((TagName="Item.Highlight"),(TagName="Item.Interactive")))`
      (`PrimitiveComponent.SetMaterial` _staticmesh 0 (`|ConvertAsset` (`self.MetalRef`))))
    (:`(GameplayTags=((TagName="Item.Collectable"),(TagName="Item.Highlight"),(TagName="Item.Interactive")))`
      (`PrimitiveComponent.SetMaterial` _staticmesh 0 (`|ConvertAsset` (`self.GoldRef`))))))