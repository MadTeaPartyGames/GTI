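; Collectible key pickup for the GTI demo that grants a colored key gameplay tag to the collecting player.
; The Construction Script switches on the last TagContainer element, using a collapsed graph to set the mesh material's Color parameter and TagToAdd for blue, green, red or yellow.
; The ItemCollectServer override passes TagToAdd to the PlayerController through AddTagMessage, then destroys the key.
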(event `/Game/GTI_Core/BPI_GTI_Interface.ItemCollectServer`
  (params (PlayerController :type "PlayerController Object Reference"))
  ;[0.2623 0 1] Event override for ItemCollectServer. Add key tag to PlayerController, then destroy.
  (message `/Game/GTI_Core/BPI_GTI_Interface.AddTag` PlayerController (`self.TagToAdd`))
  (`self.K2_DestroyActor`))

(fn `UserConstructionScript`
  ;[0.2623 0 1] Setting material color based on the Gameplay Tag specified for the key, as well as setting the tag to add to player collecting it.
  (`parent.UserConstructionScript`)
  (for _array_element (`BlueprintGameplayTagLibrary.BreakGameplayTagContainer` (`self.TagContainer`))
    _)
  (`|SwitchGameplayTag` _array_element
    (:`Item.Key.Blue`
      (`MeshComponent.SetVectorParameterValueOnMaterials` (`self.StaticMesh`) "Color" (`KismetMathLibrary.Conv_LinearColorToVector` (struct :`B` 1.0 :`A` 1.0)))
      (set `self.TagToAdd` (struct :`TagName` "Item.Key.Blue")))
    (:`Item.Key.Green`
      (`MeshComponent.SetVectorParameterValueOnMaterials` (`self.StaticMesh`) "Color" (`KismetMathLibrary.Conv_LinearColorToVector` (struct :`R` 0.006593 :`G` 1.0 :`A` 1.0)))
      (set `self.TagToAdd` (struct :`TagName` "Item.Key.Green")))
    (:`Item.Key.Red`
      (`MeshComponent.SetVectorParameterValueOnMaterials` (`self.StaticMesh`) "Color" (`KismetMathLibrary.Conv_LinearColorToVector` (struct :`R` 1.0 :`G` 0.021061 :`A` 1.0)))
      (set `self.TagToAdd` (struct :`TagName` "Item.Key.Red")))
    (:`Item.Key.Yellow`
      (`MeshComponent.SetVectorParameterValueOnMaterials` (`self.StaticMesh`) "Color" (`KismetMathLibrary.Conv_LinearColorToVector` (struct :`R` 1.0 :`G` 0.916063 :`A` 1.0)))
      (set `self.TagToAdd` (struct :`TagName` "Item.Key.Yellow")))))