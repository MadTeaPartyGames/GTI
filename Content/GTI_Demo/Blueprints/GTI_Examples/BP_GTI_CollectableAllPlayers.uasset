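; BP_GTI_CollectableAllPlayers is a GTI demo collectable that grants a tag to every player when it is collected.
; On BeginPlay it binds a handler to the server-side item-collect event and applies the gold material to its static mesh.
; The handler loops over all BP_GTI_PlayerController actors and calls AddTagMessage on each with TagToAdd.
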(event `self.ReceiveBeginPlay`
  (add `self.OnItemCollectServer` (delegate `AddTagAllPlayers`))
  (`PrimitiveComponent.SetMaterial` (`self.StaticMesh`) 0 (`|ConvertAsset` (`self.GoldRef`))))

(event `AddTagAllPlayers`
  (bind _outactors (`GameplayStatics.GetAllActorsOfClass` "/Game/GTI_Demo/Blueprints/BP_GTI_PlayerController.BP_GTI_PlayerController_C"))
  (for _array_element _outactors
    (message `/Game/GTI_Core/BPI_GTI_Interface.AddTag` _array_element (`self.TagToAdd`))))

(fn `UserConstructionScript`
  (`parent.UserConstructionScript`))